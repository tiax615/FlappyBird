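; Player pawn for a Flappy Bird game, which also drives obstacle spawning and creates the score UI.
; On BeginPlay it adds the score widget to the viewport and starts a looping timer that spawns BP_Cube at a random height.
; Left click or Space zeroes the physics Sphere's velocity, then applies an upward impulse for a consistent flap.
; Any hit on the Sphere restarts the game by opening the FlappyBird level.
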(event OnComponentHit(Sphere)
  (params (HitComponent :type Primitive%20Component%20Object%20Reference) (OtherActor :type Actor%20Object%20Reference) (OtherComp :type Primitive%20Component%20Object%20Reference) (NormalImpulse :type Vector :default "0, 0, 0") (Hit :type Hit%20Result%20Structure%20%28by%20ref%29))
  (Game|OpenLevel(byName) "FlappyBird"))

(event Custom|CreateCube
  ;[1 1 1] Create Cube
  (Game|SpawnActorfromClass "/Game/FlappyBird/BP_Cube.BP_Cube_C" (Math|Transform|MakeTransform (Math|Vector|MakeVector 0.0 1.5e+03 (Math|Random|RandomFloatinRange -3e+02 3e+02))) "Undefined" 0 0))

(event EventBeginPlay
  ;[1 1 1] Create Cube
  (Utilities|Time|SetTimerbyEvent (delegate Custom|CreateCube) 2.0 true)
  ;[1 1 1] UI Score
  (bind _returnvalue (UserInterface|CreateWidget "/Game/FlappyBird/UI_Score.UI_Score_C"))
  (UserInterface|Viewport|AddtoViewport _returnvalue 0))

(event Collision|EventActorBeginOverlap
  (params (OtherActor :type Actor%20Object%20Reference)))

(event EventTick
  (params (DeltaSeconds :type Float%20%28single-precision%29)))

(event Input|MouseEvents|LeftMouseButton
  (params (Key :type Key%20Structure :default "None"))
  (bind _sphere (Variables|Default|GetSphere))
  ;[1 1 1] Fly up
  (:Pressed
    (Physics|SetPhysicsLinearVelocity _sphere "0, 0, 0" false "None")
    (Physics|AddImpulse _sphere "0, 0,60000.000000" "None" false)))

(event Input|KeyboardEvents|SpaceBar
  (params (Key :type Key%20Structure :default "None"))
  (bind _sphere (Variables|Default|GetSphere))
  ;[1 1 1] Fly up
  (:Pressed
    (Physics|SetPhysicsLinearVelocity _sphere "0, 0, 0" false "None")
    (Physics|AddImpulse _sphere "0, 0,60000.000000" "None" false)))

(fn ConstructionScript)
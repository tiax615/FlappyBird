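; BP_Cube is an actor in a Flappy Bird game that scrolls left and awards the player a point.
; Each tick it offsets itself along local Y by Speed scaled by delta time, without sweeping.
; When its world Y drops below a fixed threshold, a DoOnce casts the player pawn to BP_BirdPawn and increments Score, so each cube scores once.
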(event EventBeginPlay)

(event Collision|EventActorBeginOverlap
  (params (OtherActor :type Actor%20Object%20Reference)))

(event EventTick
  (params (DeltaSeconds :type Float%20%28single-precision%29))
  ;[1 1 1] Move Left
  (Transformation|AddActorLocalOffset (Math|Vector|MakeVector 0.0 (* DeltaSeconds (Variables|Default|GetSpeed)) 0.0) false false)
  ;[1 1 1] Add Score
  (if (< (.Y (Math|Vector|BreakVector (Transformation|GetActorLocation))) 1e+02)
    (Utilities|FlowControl|DoOnce false
      (:Completed
        (bind _asbp_bird_pawn (Utilities|Casting|CastToBP_BirdPawn (Game|Player|GetPlayerPawn 0)))
        (Math|Integer|IncrementInt (Variables|/Game/FlappyBird/BP_BirdPawn.BP_BirdPawn_C|GetScore _asbp_bird_pawn))))))

(fn ConstructionScript)